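; Lift actor that moves vertically between its placed position and an offset scaled by LiftHeight.
; Tick polls an optional Trigger reference and, once it is activated, destroys it and calls MoveLift.
; MoveLift plays or reverses a timeline that drives Z from the StartLocation cached in the construction script.
; SwitchDirection flips when the timeline finishes, so the next MoveLift call travels the opposite way.
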(event `self.ReceiveTick`
  (params (DeltaSeconds :type "Float (single-precision)"))
  (bind _trigger (`self.Trigger`))
  ;[1 1 1] Check for open or close triggers
  (if (`KismetSystemLibrary.IsValid` _trigger)
    (if (`/Game/Blueprints/InvisibleTriggerBP.trigger` _trigger)
      (`self.K2_DestroyActor` _trigger) ; destroys the trigger to prevent player from reopening door
      (`self.MoveLift`))))

(event `MoveLift`
  ;[1 1 1] Open
  (if (`self.switchDirection`)
    (bind (_direction _newtrack_1) (`Timeline|Timeline_0` :!via `Reverse` :!label _label)
      (:`Update`
        (`self.K2_SetActorLocation` (+ (`KismetMathLibrary.MakeVector` 0.0 0.0 (* _newtrack_1 (`self.LiftHeight`))) (`self.startLocation`))))
      (:`Finished`
        (if (`self.switchDirection`)
          (set `self.switchDirection` false)
          (else
            (set `self.switchDirection` true)))))
    (else
      (goto _label))))

(fn `UserConstructionScript`
  (set `self.startLocation` (`self.K2_GetActorLocation`)))