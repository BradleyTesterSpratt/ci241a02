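; Enemy pawn that walks to a waypoint, then chases and shoots the player once PawnSensing spots them.
; Each sighting updates the destination, turns the enemy with a fixed Y aim offset and spawns a projectile from the Sphere; Tick issues AIMoveTo toward the destination.
; Overlapping normal or super projectiles subtract their Strength from Health; at zero it destroys itself and spawns its held object's class.
; Attack is an empty stub.
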(event `self.ReceiveActorBeginOverlap`
  (params (OtherActor :type "Actor Object Reference"))
  (bind _output_get (set `self.collidedActor` OtherActor))
  (bind _asfirst_person_projectile (cast `/Game/Blueprints/FirstPersonProjectile` (`self.collidedActor`))
    (:`then`
      (`self.takeDamage` (`/Game/Blueprints/FirstPersonProjectile.Strength` _asfirst_person_projectile)))
    (:`CastFailed`
      (bind _asfirst_person_super_projectile (cast `/Game/Blueprints/FirstPersonSuperProjectile` (`self.collidedActor`)))
      (`self.takeDamage` (`/Game/Blueprints/FirstPersonSuperProjectile.Strength` _asfirst_person_super_projectile))))
  (`self.checkDeath`))

(event `self.PawnSensing.OnSeePawn`
  (params (Pawn :type "Pawn Object Reference"))
  (bind _asfirst_person_character (cast `/Game/Blueprints/FirstPersonCharacter` Pawn))
  (set `self.Destination` (`self.K2_GetActorLocation` _asfirst_person_character))
  (`|ExecutionSequence`
    (:`then_0`
      (`self.lookAt` (`self.Destination`)))
    (:`then_1`
      (`|SpawnActorFromClass` "/Game/Blueprints/FirstPersonProjectile.FirstPersonProjectile_C" (`SceneComponent.K2_GetComponentToWorld` (`self.sphere`)) "Undefined" "OverrideRootScale" null null))))

(event `self.ReceiveTick`
  (params (DeltaSeconds :type "Float (single-precision)"))
  (bind _destination (`self.Destination`))
  (if (not (== _destination (`self.K2_GetActorLocation`) :`ErrorTolerance` 0.005))
    (`|AIMoveTo` self _destination)))

(fn `attack`)

(fn `checkDeath`
  (bind _heldobject (`self.HeldObject`))
  (if (<= (`self.Health`) 0)
    (`self.K2_DestroyActor`)
    ;[1 1 1] If held object is set, drop it
    (`/Engine/EditorBlueprintResources/StandardMacros.IsValid` _heldobject
      (:`Is Valid`
        (`|SpawnActorFromClass` (`GameplayStatics.GetObjectClass` _heldobject) (`self.GetTransform`) "Undefined" "OverrideRootScale" null null)))))

(fn `lookAt`
  (params (LookDestination :type "Vector Structure"))
  (`self.K2_SetActorRotation` (`KismetMathLibrary.FindLookAtRotation` (`self.K2_GetActorLocation`) (`KismetMathLibrary.MakeVector` (.x LookDestination) (+ (.y LookDestination) 140.0) (.z (`self.K2_GetActorLocation`))))))

(fn `takeDamage`
  (params (damage :type Integer))
  (set `self.Health` (- (`self.Health`) damage)))

(fn `UserConstructionScript`
  (set `self.Destination` (`self.K2_GetActorLocation` (`self.Waypoint`)))
  (`SceneComponent.K2_AttachToComponent` (`self.SkeletalMesh`) (`self.Mesh`) "GunSocket" "SnapToTarget" "SnapToTarget" "SnapToTarget" true))