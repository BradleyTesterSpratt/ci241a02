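; giBP holds shared player state: health, armour, super ammo, green keys and an on-screen help message.
; Safe-space saves snapshot location, health, armour and ammo, which RespawnPlayer restores, returning the location; keys are not saved.
; Damage hits armour while any remains, with no overflow into health, and returns whether health is depleted.
; Key and ammo checks consume one item on success or set the help message on failure.
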(fn `AmmoCheck`
  (returns (CanFire :type Boolean))
  (locals (`can Fire` :type Boolean))
  (bind _output_get (set `local.can Fire` (> (`self.SuperAmmo`) 0)))
  (if _output_get
    (`/Engine/EditorBlueprintResources/StandardMacros.DecrementInt` (`self.SuperAmmo`)
      (:`  `
        _))
    (else
      (set `self.HelpMessage` "Not Enough Ammo")))
  (return (`local.can Fire`)))

(fn `ClearMessage`
  (set `self.HelpMessage` " "))

(fn `PlayerTakeFire`
  (params (incomingDamage :type Integer))
  (returns (isDead :type Boolean))
  (locals (Damage :type Integer))
  (bind _playerarmour (`self.PlayerArmour`))
  (bind _damage (`local.Damage`))
  (set `local.Damage` incomingDamage)
  (if (> _playerarmour 0)
    (set `self.PlayerArmour` (- _playerarmour _damage))
    (else
      (bind _output_get (set `self.PlayerHealth` (- (`self.PlayerHealth`) _damage)))))
  (return (<= _output_get 0)))

(fn `RespawnPlayer`
  (returns (RespawnLocation :type "Vector Structure"))
  (set `self.SuperAmmo` (`self.respawnSuperAmmo`))
  (set `self.PlayerHealth` (`self.RespawnHealth`))
  (set `self.PlayerArmour` (`self.RespawnArmour`))
  (return (`self.RespawnLocation`)))

(fn `SetHelpMessage`
  (params (NewParam :type String))
  (set `self.HelpMessage` NewParam))

(fn `SetLastSafeSpace`
  (params (CurrentLocation :type "Vector Structure"))
  (set `self.RespawnLocation` CurrentLocation)
  (set `self.RespawnArmour` (`self.PlayerArmour`))
  (set `self.RespawnHealth` (`self.PlayerHealth`))
  (set `self.respawnSuperAmmo` (`self.SuperAmmo`)))

(fn `UseKey`
  (returns (OpenDoor :type Boolean))
  (locals (`Open Door` :type Boolean))
  (bind _output_get (set `local.Open Door` (> (`self.GreenKeys`) 0)))
  (if _output_get
    (`/Engine/EditorBlueprintResources/StandardMacros.DecrementInt` (`self.GreenKeys`)
      (:`  `
        _))
    (else
      (set `self.HelpMessage` "\"You need a key\"")))
  (return (`local.Open Door`)))