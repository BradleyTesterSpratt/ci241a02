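; Sliding door actor that moves vertically between its start location and a DoorHeight offset, optionally starting open.
; Tick polls an optional invisible trigger, which can require a green key from the giBP game instance, and an optional pressure plate.
; A successful trigger is destroyed to prevent reuse.
; Both inputs call ToggleDoor, which plays or reverses a timeline and flips SwitchDirection when it finishes.
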(event `self.ReceiveTick`
  (params (DeltaSeconds :type "Float (single-precision)"))
  (bind _plate (`self.Plate`))
  (bind _trigger (`self.Trigger`))
  ;[1 1 1] Check for open or close triggers
  (if (`KismetSystemLibrary.IsValid` _trigger)
    (if (`/Game/Blueprints/InvisibleTriggerBP.trigger` _trigger)
      (if (`self.RequiresGreenKey`)
        (bind _asgi_bp (cast `/Game/Blueprints/giBP` (`GameplayStatics.GetGameInstance`)))
        (bind _opendoor (`/Game/Blueprints/giBP.UseKey` _asgi_bp))
        (if _opendoor
          (`self.K2_DestroyActor` _trigger :!label _label) ; destroys the trigger to prevent player from reopening door
          (`self.toggleDoor` :!label _label_2) ; open or close the door
          (else
            (`KismetSystemLibrary.Delay` 1.5)
            (`/Game/Blueprints/giBP.ClearMessage` _asgi_bp)))
        (else
          (goto _label)))
      (else
        (if (`KismetSystemLibrary.IsValid` _plate) :!label _label_3
          (if (`/Game/Blueprints/PressurePlateBP.Trigger` _plate)
            (goto _label_2)))))
    (else
      (goto _label_3))))

(event `self.ReceiveBeginPlay`
  (`self.setStartState`))

(event `toggleDoor`
  ;[1 1 1] Open/Close Door
  (if (`self.switchDirection`)
    (bind (_direction _newtrack_1) (`Timeline|toggleDoorTL` :!via `Reverse` :!label _label_4)
      (:`Update`
        (`self.K2_SetActorLocation` (+ (`KismetMathLibrary.MakeVector` 0.0 0.0 (* _newtrack_1 (`self.DoorHeight`))) (`self.startLoc`))))
      (:`Finished`
        (if (`self.switchDirection`)
          (set `self.switchDirection` false)
          (else
            (set `self.switchDirection` true)))))
    (else
      (goto _label_4))))

(fn `setStartState`
  (set `self.startLoc` (`self.K2_GetActorLocation`))
  (if (`self.StartOpen`)
    (`self.toggleDoor`)))

(fn `UserConstructionScript`)