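; AmmoBP is an ammo pickup that grants super ammo when FirstPersonCharacter overlaps it.
; On overlap it destroys itself, then increases the SuperAmmo count stored in the giBP game instance.
; Until FirstAmmoPickup is set, it also shows an ammo-switch hint through the game instance.
; Clearing the hint and setting that flag follow a Delay on the already destroyed actor.
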(event `self.ReceiveActorBeginOverlap`
  (params (OtherActor :type "Actor Object Reference"))
  (if (== (`GameplayStatics.GetObjectClass` OtherActor) "/Game/Blueprints/FirstPersonCharacter.FirstPersonCharacter_C")
    (`self.K2_DestroyActor`)
    (bind _asgi_bp (cast `/Game/Blueprints/giBP` (`GameplayStatics.GetGameInstance`)))
    (set `/Game/Blueprints/giBP.SuperAmmo` (+ (`/Game/Blueprints/giBP.SuperAmmo` _asgi_bp) 10) _asgi_bp)
    (if (not (`/Game/Blueprints/giBP.firstAmmoPickup` _asgi_bp))
      (`/Game/Blueprints/giBP.SetHelpMessage` _asgi_bp "Right Click To Change Ammo Type")
      (`KismetSystemLibrary.Delay` 1.5)
      (`/Game/Blueprints/giBP.ClearMessage` _asgi_bp)
      (set `/Game/Blueprints/giBP.firstAmmoPickup` true _asgi_bp))))

(fn `UserConstructionScript`)