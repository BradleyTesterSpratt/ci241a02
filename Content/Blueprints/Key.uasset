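; Key pickup actor that adds a green key to the player's count.
; It spins continuously around its vertical axis each tick at a fixed per-frame rate.
; When an actor of exactly the FirstPersonCharacter class overlaps it, it destroys itself and increments GreenKeys on the giBP game instance, which holds the count.
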(event `self.ReceiveTick`
  (params (DeltaSeconds :type "Float (single-precision)"))
  (`self.K2_AddActorWorldRotation` (struct :`Yaw` 2.5)))

(event `self.ReceiveActorBeginOverlap`
  (params (OtherActor :type "Actor Object Reference"))
  (if (== (`GameplayStatics.GetObjectClass` OtherActor) "/Game/Blueprints/FirstPersonCharacter.FirstPersonCharacter_C")
    (`self.K2_DestroyActor`)
    (bind _asgi_bp (cast `/Game/Blueprints/giBP` (`GameplayStatics.GetGameInstance`)))
    (bind _result (`/Engine/EditorBlueprintResources/StandardMacros.IncrementInt` (`/Game/Blueprints/giBP.GreenKeys` _asgi_bp))
      (:`  `
        (set `/Game/Blueprints/giBP.GreenKeys` _result _asgi_bp)))))

(fn `UserConstructionScript`)